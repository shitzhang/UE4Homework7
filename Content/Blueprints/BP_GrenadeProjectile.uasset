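; BP_GrenadeProjectile is a grenade projectile Blueprint holding explosion logic that is currently disconnected, so none of it runs.
; The unwired nodes outline a one-second fuse calling Explode, plus a chain spawning an explosion effect and applying full radial damage credited to the instigator.
; That chain also fires a RadialForceComp impulse, sharing its radius with damage and a debug sphere, then destroys the actor.
; BeginPlay and the construction script are empty.
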(event `self.ReceiveBeginPlay`)

(fn `UserConstructionScript`)